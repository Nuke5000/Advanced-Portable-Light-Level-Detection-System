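; BoyGuard_BP is a guard that reacts to how brightly lit the player character is, currently only through on-screen debug text.
; BeginPlay finds and caches the ThirdPersonCharacter.
; Tick reads LitPercentAllLights from the character's APLLDSComponentBP and prints one of three alert lines by light band, from suspicion to detection.
; The check uses light level alone, with no distance or line-of-sight test.
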(event EventBeginPlay
  (bind _returnvalue (Actor|GetActorOfClass "/Game/ThirdPersonCPP/Blueprints/ThirdPersonCharacter.ThirdPersonCharacter_C"))
  (bind _asthird_person_character (Utilities|Casting|CastToThirdPersonCharacter _returnvalue)))

(event Collision|EventActorBeginOverlap
  (params (OtherActor :type Actor%20Object%20Reference)))

(event EventTick
  (params (DeltaSeconds :type Float%20%28single-precision%29))
  (if (> (Variables|/Script/Game.APLLDS_Component|GetLit_Percent_AllLights (Variables|/Game/ThirdPersonCPP/Blueprints/ThirdPersonCharacter.ThirdPersonCharacter_C|GetAPLLDS_Component_BP (stale EventBeginPlay _asthird_person_character))) 5e+01)
    (Development|PrintString "Guard: I SEE YOU!" true true "(R=0.840210,G=0.185400,B=0.000000,A=1.000000)" 0.01)
    (elif (and (< (Variables|/Script/Game.APLLDS_Component|GetLit_Percent_AllLights (Variables|/Game/ThirdPersonCPP/Blueprints/ThirdPersonCharacter.ThirdPersonCharacter_C|GetAPLLDS_Component_BP (stale EventBeginPlay _asthird_person_character))) 5e+01) (> (Variables|/Script/Game.APLLDS_Component|GetLit_Percent_AllLights (Variables|/Game/ThirdPersonCPP/Blueprints/ThirdPersonCharacter.ThirdPersonCharacter_C|GetAPLLDS_Component_BP (stale EventBeginPlay _asthird_person_character))) 4e+01))
      (Development|PrintString "Guard: Is someone there?" true true "(R=0.840210,G=0.185400,B=0.000000,A=1.000000)" 0.01)
      (elif (and (< (Variables|/Script/Game.APLLDS_Component|GetLit_Percent_AllLights (Variables|/Game/ThirdPersonCPP/Blueprints/ThirdPersonCharacter.ThirdPersonCharacter_C|GetAPLLDS_Component_BP (stale EventBeginPlay _asthird_person_character))) 4e+01) (> (Variables|/Script/Game.APLLDS_Component|GetLit_Percent_AllLights (Variables|/Game/ThirdPersonCPP/Blueprints/ThirdPersonCharacter.ThirdPersonCharacter_C|GetAPLLDS_Component_BP (stale EventBeginPlay _asthird_person_character))) 3e+01))
        (Development|PrintString "Guard: What was that?" true true "(R=0.840210,G=0.185400,B=0.000000,A=1.000000)" 0.01)))))

(fn ConstructionScript)