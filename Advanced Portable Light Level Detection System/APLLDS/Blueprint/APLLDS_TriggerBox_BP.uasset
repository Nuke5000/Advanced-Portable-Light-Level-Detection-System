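; A trigger box that overrides the player's light level detection (APLLDS) settings while the ThirdPersonCharacter is inside it.
; On begin overlap it saves the component's level modifier, sets a fixed modifier, zeroes the non-falloff light percent and prints debug messages.
; On end overlap it restores the saved modifier, but resets the light percent to zero rather than restoring its previous value.
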(event OnComponentBeginOverlap(TriggerBox)
  (params (OverlappedComponent :type Primitive%20Component%20Object%20Reference) (OtherActor :type Actor%20Object%20Reference) (OtherComp :type Primitive%20Component%20Object%20Reference) (OtherBodyIndex :type Integer) (bFromSweep :type Boolean) (SweepResult :type Hit%20Result%20Structure%20%28by%20ref%29))
  ;[1 1 1] Overlap begins to change LLDS modifier
  (bind _returnvalue (Actor|GetActorOfClass "/Game/ThirdPersonCPP/Blueprints/ThirdPersonCharacter.ThirdPersonCharacter_C"))
  (bind _asthird_person_character (Utilities|Casting|CastToThirdPersonCharacter _returnvalue))
  (if (== OtherActor _asthird_person_character)
    (Development|PrintString "Player Overlapped" true true "(R=0.000000,G=0.660000,B=1.000000,A=1.000000)" 2e+01)
    (Variables|Default|SetAPLLDS%20Modifier%20Original%20Value (Variables|/Script/Game.APLLDS_Component|GetAPLLDS_Level_Modifier (Variables|/Game/ThirdPersonCPP/Blueprints/ThirdPersonCharacter.ThirdPersonCharacter_C|GetAPLLDS_Component_BP _asthird_person_character)))
    ;[1 1 1] The two most important values
    (Variables|/Script/Game.APLLDS_Component|SetAPLLDS_Level_Modifier (Variables|/Game/ThirdPersonCPP/Blueprints/ThirdPersonCharacter.ThirdPersonCharacter_C|GetAPLLDS_Component_BP _asthird_person_character) 1.0)
    (bind _output_get (Variables|/Script/Game.APLLDS_Component|SetNon_Falloff_Light_Percent (Variables|/Game/ThirdPersonCPP/Blueprints/ThirdPersonCharacter.ThirdPersonCharacter_C|GetAPLLDS_Component_BP _asthird_person_character) 0.0))
    (Development|PrintString "Lit Percent ALl Lights has been manually adjust by:" true true "(R=0.441447,G=0.000000,B=0.380966,A=1.000000)" 1e+01)
    (Development|PrintString (Utilities|String|ToString(Float) _output_get) true true "(R=0.441447,G=0.000000,B=0.380966,A=1.000000)" 1e+01)))

(event OnComponentEndOverlap(TriggerBox)
  (params (OverlappedComponent :type Primitive%20Component%20Object%20Reference) (OtherActor :type Actor%20Object%20Reference) (OtherComp :type Primitive%20Component%20Object%20Reference) (OtherBodyIndex :type Integer))
  ;[1 1 1] Overlap ends to change the LLDS modifier back to normal
  (bind _returnvalue (Actor|GetActorOfClass "/Game/ThirdPersonCPP/Blueprints/ThirdPersonCharacter.ThirdPersonCharacter_C"))
  (bind _asthird_person_character (Utilities|Casting|CastToThirdPersonCharacter _returnvalue))
  (if (== _asthird_person_character OtherActor)
    (Development|PrintString "Player Overlap Ended" true true "(R=0.000000,G=0.660000,B=1.000000,A=1.000000)" 2e+01)
    ;[1 1 1] The two most important values
    (Variables|/Script/Game.APLLDS_Component|SetAPLLDS_Level_Modifier (Variables|/Game/ThirdPersonCPP/Blueprints/ThirdPersonCharacter.ThirdPersonCharacter_C|GetAPLLDS_Component_BP _asthird_person_character) (Variables|Default|GetAPLLDS%20Modifier%20Original%20Value))
    (Variables|/Script/Game.APLLDS_Component|SetNon_Falloff_Light_Percent (Variables|/Game/ThirdPersonCPP/Blueprints/ThirdPersonCharacter.ThirdPersonCharacter_C|GetAPLLDS_Component_BP _asthird_person_character) 0.0)))

(fn ConstructionScript)