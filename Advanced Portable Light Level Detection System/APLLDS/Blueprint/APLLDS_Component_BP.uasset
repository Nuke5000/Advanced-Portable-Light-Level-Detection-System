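; Blueprint component for the APLLDS light level detection system, bridging its C++ logic with actor and light data.
; The APLLDS event finds the CharacterEditor and ThirdPersonCharacter, then passes the former's location and the latter's mesh rotation to GetLightLevel.
; C++-called events copy rect and spot light attenuation radii into variables and apply a stored falloff exponent to spot lights.
; Disconnected debug prints remain for testing.
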(event Custom|APLLDS
  (bind _returnvalue (Actor|GetActorOfClass (Variables|Default|GetCharacter_Editor)))
  (bind _returnvalue_2 (Actor|GetActorOfClass "/Game/ThirdPersonCPP/Blueprints/ThirdPersonCharacter.ThirdPersonCharacter_C"))
  (bind _asthird_person_character (Utilities|Casting|CastToThirdPersonCharacter _returnvalue_2))
  (Class|APLLDSComponent|GetLightLevel (Transformation|GetActorLocation _returnvalue) (Transformation|GetWorldRotation (Variables|/Script/Engine.Character|GetMesh _asthird_person_character))))

(event EventSetRectLightRadius
  (params (LightComp :type Rect%20Light%20Component%20Object%20Reference))
  ;[1 1 1] Spot Light C++ to BP Function Calls
  (bind _output_get (Variables|Default|SetRectLight_LightRadius (Variables|/Script/Engine.LocalLightComponent|GetAttenuationRadius LightComp))))

(event EventSetSpotLightRadius
  (params (LightComp :type Spot%20Light%20Component%20Object%20Reference))
  ;[1 1 1] Spot Light C++ to BP Function Calls
  (bind _output_get (Variables|Default|SetSpotLight_LightRadius (Variables|/Script/Engine.LocalLightComponent|GetAttenuationRadius LightComp))))

(event EventSetSpotLightLightFalloffExponent
  (params (LightComp :type Spot%20Light%20Component%20Object%20Reference))
  ;[1 1 1] Spot Light C++ to BP Function Calls
  (Class|PointLightComponent|SetLightFalloffExponent LightComp (Variables|Default|GetSpotLight_LightFalloffExponent)))